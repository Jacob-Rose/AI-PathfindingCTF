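; BP_SteeringActor provides debug visuals for a steering actor's velocity and path.
; UpdateArrow stretches the Arrow along X as the SteeringVelocity magnitude rises toward MaxSpeed, using a clamped range mapping.
; DisplatPath draws debug spheres at TargetPos and at each point in Path.
; The construction script is empty, and neither the steering logic nor any calls to these functions appear here.
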(fn ConstructionScript)

(fn UpdateArrow
  (Transformation|SetRelativeScale3D (Variables|Default|GetArrow) (Math|Vector|MakeVector (Math|Float|MapRangeClamped (Math|Vector|VectorLength (Variables|Default|GetSteeringVelocity)) 0.0 (Variables|Default|GetMaxSpeed) 1.0 3.0) 2.0 3.0)))

(fn DisplatPath
  (Rendering|Debug|DrawDebugSphere (Variables|Default|GetTargetPos) 1e+02 12 "(R=0.117766,G=1.000000,B=0.143879,A=1.000000)" 0.0)
  (for _array_element (Variables|Default|GetPath)
    (Rendering|Debug|DrawDebugSphere _array_element 3e+01 12 "(R=0.356519,G=1.000000,B=0.617714,A=1.000000)" 0.0)))